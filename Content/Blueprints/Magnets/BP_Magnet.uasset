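; BP_Magnet is a physics-driven magnet actor with switchable polarity that triggers Game Over on BP_PlayerController when it hits another magnet.
; Its Magnetic component supplies a force each magnetic tick, applied at the cube's center of mass alongside sideways movement from MoveRight.
; Construction sets charge, mass and a dynamic material whose color follows polarity.
; Tick continually lerps rotation back to the orientation recorded at BeginPlay.
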(event `self.ReceiveBeginPlay`
  (set `self.DefaultRotation` (`self.K2_GetActorRotation`))
  (`self.SetupColor`))

(event `self.Magnetic.MagneticTick`
  (params (MagneticForce :type "Vector Structure") (DeltaTime :type "Float (single-precision)"))
  (`self.AddForce` MagneticForce))

(event `self.ReceiveTick`
  (params (DeltaSeconds :type "Float (single-precision)"))
  (`self.RotateBack` DeltaSeconds 10.0))

(event `self.Cube.OnComponentHit`
  (params (HitComponent :type "PrimitiveComponent Object Reference") (OtherActor :type "Actor Object Reference") (OtherComp :type "PrimitiveComponent Object Reference") (NormalImpulse :type "Vector Structure") (Hit :type "HitResult Structure (by ref)"))
  (cast `/Game/Blueprints/Magnets/BP_Magnet` OtherActor)
  (bind _asbp_player_controller (cast `/Game/Blueprints/Player/BP_PlayerController` (`GameplayStatics.GetPlayerController` 0)))
  (`/Game/Blueprints/Player/BP_PlayerController.GameOver` _asbp_player_controller))

(fn `AddForce`
  (params (InputPin :type "Vector Structure"))
  (bind _componenttoupdate (`self.GetUpdatedComponent`))
  (`PrimitiveComponent.AddForceAtLocation` _componenttoupdate InputPin (`PrimitiveComponent.GetCenterOfMass` _componenttoupdate "None") "None"))

(fn `GetUpdatedComponent`
  (returns (ComponentToUpdate :type "PrimitiveComponent Object Reference"))
  (return (`self.Cube`)))

(fn `Move Right`
  (params (Y :type "Float (double-precision)"))
  (`self.AddForce` (`KismetMathLibrary.MakeVector` 0.0 (* Y (`self.RightMoveScale`)))))

(fn `RotateBack`
  (params (Alpha :type "Float (double-precision)") (Speed :type "Float (double-precision)"))
  (`self.K2_SetActorRotation` (`KismetMathLibrary.RLerp` (`self.K2_GetActorRotation`) (`self.DefaultRotation`) (* Alpha Speed) true) true))

(fn `SetPolarity`
  (params (Positive :type Boolean))
  (`|ExecutionSequence`
    (:`then_0`
      (set `MagneticComponent.IsPositive` Positive (`self.Magnetic`)))
    (:`then_1`
      (`/Engine/EditorBlueprintResources/StandardMacros.IsValid` (`self.MagnetMaterial`)
        (:`Is Valid`
          (`MaterialInstanceDynamic.SetVectorParameterValue` (`self.MagnetMaterial`) "Color" (select `bool` Positive :`false` (`self.NegativeColor`) :`true` (`self.PositiveColor`))))
        (:`Is Not Valid`
          (`KismetSystemLibrary.PrintString` "Error Invalid Material"))))))

(fn `Setup`
  (set `MagneticComponent.Charge` (* (`self.Charge`) 100.0) (`self.Magnetic`))
  (`PrimitiveComponent.SetMassOverrideInKg` (`self.GetUpdatedComponent`) "None" (`self.Mass`) true)
  (`self.SetupColor`))

(fn `SetupColor`
  (bind _returnvalue (`PrimitiveComponent.CreateDynamicMaterialInstance` (`self.Cube`) 0 "/Game/Material/M_Magnets.M_Magnets" "None"))
  (set `self.MagnetMaterial` _returnvalue)
  (`self.SetPolarity` (`MagneticComponent.IsPositive` (`self.Magnetic`))))

(fn `TogglePolarity`
  (`self.SetPolarity` (not (`MagneticComponent.IsPositive` (`self.Magnetic`)))))

(fn `UserConstructionScript`
  (`self.Setup`))