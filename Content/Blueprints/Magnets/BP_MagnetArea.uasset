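; BP_MagnetArea is a box-bounded area that ends the game when a magnet leaves it.
; The Box end-overlap event checks whether the departing actor casts to BP_Magnet, then calls GameOver, which forwards to BP_GameInstance's GoToGameOver.
; An IsSuccess function returns the IsFail variable directly, though nothing in this graph sets that variable or calls the function.
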(event `self.Box.OnComponentEndOverlap`
  (params (OverlappedComponent :type "PrimitiveComponent Object Reference") (OtherActor :type "Actor Object Reference") (OtherComp :type "PrimitiveComponent Object Reference") (OtherBodyIndex :type Integer))
  ;[1 1 1] Detect Magnet leaving
  (if (`self.IsMagnet` OtherActor)
    (`self.GameOver`)))

(fn `GameOver`
  (bind _asbp_game_instance (cast `/Game/Blueprints/Game/BP_GameInstance` (`GameplayStatics.GetGameInstance`)))
  (`/Game/Blueprints/Game/BP_GameInstance.GoToGameOver` _asbp_game_instance))

(fn `IsMagnet`
  (params (InActor :type "Actor Object Reference"))
  (returns (IsMagnet :type Boolean))
  (cast `/Game/Blueprints/Magnets/BP_Magnet` InActor
    (:`then`
      (return true))
    (:`CastFailed`
      (return false))))

(fn `IsSuccess`
  (returns (bIsSuccess :type Boolean))
  (return (`self.bIsFail`)))

(fn `UserConstructionScript`)