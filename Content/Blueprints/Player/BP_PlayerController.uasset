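; Player controller that tracks level completion and drives level transitions through the game instance.
; On begin play it caches all BP_MagnetTarget actors and the BP_GameInstance.
; Each tick it checks whether every target reports success and, if so, asks the game instance to load the next level.
; The ResetLevel input restarts the level, and a GameOver event forwards to the game instance's game over flow.
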(event `self.ReceiveBeginPlay`
  (`self.Setup`))

(event `self.ReceiveTick`
  (params (DeltaSeconds :type "Float (single-precision)"))
  (if (`self.LevelComplete`)
    (`/Game/Blueprints/Game/BP_GameInstance.GoToNextLevel` (`self.GameInstance`))))

(event `InputAction|ResetLevel`
  (params (Key :type "Key Structure"))
  (:`Pressed`
    (`/Game/Blueprints/Game/BP_GameInstance.GoToRestartLevel` (`self.GameInstance`))))

(event `GameOver`
  (`/Game/Blueprints/Game/BP_GameInstance.GoToGameOver` (`self.GameInstance`)))

(fn `LevelComplete`
  (returns (Success :type Boolean))
  (locals (IsSuccess :type Boolean :default false))
  (set `local.IsSuccess` true)
  (for _array_element (`self.Targets`)
    (set `local.IsSuccess` (and (`/Game/Blueprints/Magnets/BP_MagnetTarget.IsSuccess` _array_element) (`local.IsSuccess`))))
  (return (`local.IsSuccess`)))

(fn `Setup`
  (bind _outactors (`GameplayStatics.GetAllActorsOfClass` "/Game/Blueprints/Magnets/BP_MagnetTarget.BP_MagnetTarget_C"))
  (set `self.Targets` _outactors)
  (bind _asbp_game_instance (cast `/Game/Blueprints/Game/BP_GameInstance` (`GameplayStatics.GetGameInstance`)))
  (set `self.GameInstance` _asbp_game_instance))

(fn `UserConstructionScript`)