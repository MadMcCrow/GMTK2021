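; Player camera pawn that follows a group of magnets and forwards the player's input to them.
; Each tick it teleports to the magnets' average position and scales spring arm length by their mean distance from that point.
; It also nudges magnets that diverge too far on Y back toward the midpoint.
; MoveRight input moves all magnets, while ToggleMagnets flips only the first magnet's polarity, as its random range is zero.
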(event `self.ReceiveTick`
  (params (DeltaSeconds :type "Float (single-precision)"))
  (bind (_midpoint _amplitude) (`self.GetCenterOfMagnets`))
  (`|ExecutionSequence`
    (:`then_0`
      (`self.K2_SetActorLocation` _midpoint false true)
      (set `SpringArmComponent.TargetArmLength` (* _amplitude (`self.CameraDistanceFactor`)) (`self.SpringArm`)))
    (:`then_1`
      (`self.FixMagnetsPosition` _midpoint))))

(event `InputAxis|MoveRight`
  (params (AxisValue :type "Float (single-precision)"))
  ;[1 1 1] MoveMagnets
  (`self.MoveMagnetsRight` AxisValue 2.0))

(event `InputAction|ToggleMagnets`
  (params (Key :type "Key Structure"))
  (:`Pressed`
    (`self.ToggleMagnets`)))

(event `Audio_Toggle`)

(fn `FixMagnetsPosition`
  (params (`Move Target` :type "Vector Structure"))
  (for _array_element (`self.Magnets`)
    (bind _y (.y (- `Move Target` (`self.K2_GetActorLocation` _array_element))))
    (if (> (`KismetMathLibrary.Abs` _y) (`self.MaxDivergence`))
      (`/Game/Blueprints/Magnets/BP_Magnet.Move Right` _array_element (/ _y 2.0)))))

(fn `GetCenterOfMagnets`
  (returns (MidPoint :type "Vector Structure") (Amplitude :type "Float (double-precision)"))
  (locals (MagnetDistance :type "Float (double-precision)" :default 0.0))
  (bind _magnets (`self.Magnets`))
  (bind _returnvalue (`GameplayStatics.GetActorArrayAverageLocation` _magnets))
  (set `local.MagnetDistance` 0.0)
  (for _array_element _magnets
    (set `local.MagnetDistance` (+ (`local.MagnetDistance`) (`KismetMathLibrary.Vector_Distance` (`self.K2_GetActorLocation` _array_element) _returnvalue))))
  (return _returnvalue (/ (`local.MagnetDistance`) (`KismetMathLibrary.Conv_IntToDouble` (`KismetArrayLibrary.Array_Length` _magnets)))))

(fn `MoveMagnetsRight`
  (params (Y :type "Float (double-precision)") (Scale :type "Float (double-precision)"))
  (for _array_element (`self.Magnets`)
    (`/Game/Blueprints/Magnets/BP_Magnet.Move Right` _array_element (* Y Scale))))

(fn `ToggleMagnets`
  (`/Game/Blueprints/Magnets/BP_Magnet.TogglePolarity` (`|GetArrayItem` (`self.Magnets`) (`KismetMathLibrary.RandomIntegerInRange` 0))))

(fn `UserConstructionScript`)