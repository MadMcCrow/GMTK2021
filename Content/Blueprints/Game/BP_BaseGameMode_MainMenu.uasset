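; Game mode for the main menu level that shows the menu UI and handles its Start and Quit actions.
; On BeginPlay it caches BP_GameInstance, creates WBP_MainMenu, binds its start and quit events, and switches to UI-only input with a visible cursor.
; Start opens Level_1 through the game instance, and Quit exits the game.
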(event `self.ReceiveBeginPlay`
  (`|ExecutionSequence`
    (:`then_0`
      (bind _asbp_game_instance (cast `/Game/Blueprints/Game/BP_GameInstance` (`GameplayStatics.GetGameInstance`)))
      (set `self.GameInstance` _asbp_game_instance))
    (:`then_1`
      (bind _returnvalue (`|CreateWidget` "/Game/Blueprints/UI/WBP_MainMenu.WBP_MainMenu_C" (`GameplayStatics.GetPlayerController` 0)))
      (set `self.MainMenu` _returnvalue))
    (:`then_2`
      (add `/Game/Blueprints/UI/WBP_MainMenu.Quit` (`self.MainMenu`) (delegate `Quit`))
      (add `/Game/Blueprints/UI/WBP_MainMenu.Start` (`self.MainMenu`) (delegate `Start`)))
    (:`then_3`
      (`UserWidget.AddToViewport` (`self.MainMenu`) 0))
    (:`then_4`
      (`WidgetBlueprintLibrary.SetInputMode_UIOnlyEx` (`GameplayStatics.GetPlayerController` 0) (`self.MainMenu`) "LockOnCapture")
      (set `PlayerController.bShowMouseCursor` true (`GameplayStatics.GetPlayerController` 0)))))

(event `Start`
  (`LevelGameInstance.OpenLevel` (`self.GameInstance`) "/Game/Maps/Level_1.Level_1"))

(event `Quit`
  (`KismetSystemLibrary.QuitGame` null "Quit"))

(fn `UserConstructionScript`)